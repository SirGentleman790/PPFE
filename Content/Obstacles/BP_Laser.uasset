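; BP_Laser is a laser obstacle that damages the player and sends them back to a respawn point.
; A timeline started on BeginPlay moves LaserBase along the spline, using the length cached in the construction script.
; Any actor overlap applies damage to the cached player character and teleports it to the Respawn component of BPRespawn, without checking which actor overlapped.
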(event `self.ReceiveBeginPlay`
  ;[1 1 1] Ref au joueur
  (bind _asbp_third_person_character (cast `/Game/ThirdPerson/Blueprints/BP_ThirdPersonCharacter` (`GameplayStatics.GetPlayerCharacter` 0)))
  (set `self.AsPlayer` _asbp_third_person_character)
  ;[1 1 1] Timeline pour la spline
  (bind (_direction _newtrack_0) (`Timeline|mvtLaser`)
    (:`Update`
      (`SceneComponent.K2_SetRelativeLocation` (`self.LaserBase`) (`SplineComponent.GetLocationAtDistanceAlongSpline` (`self.Spline`) (* _newtrack_0 (`self.lngSpline`)) "Local") false false))))

(event `self.ReceiveActorBeginOverlap`
  (params (OtherActor :type "Actor Object Reference"))
  (bind _asplayer (`self.AsPlayer`))
  ;[1 1 1] respawn sur overlap + dégats reçus
  (`GameplayStatics.ApplyDamage` _asplayer 10.0)
  (`self.K2_TeleportTo` :`self` _asplayer :`DestLocation` (`SceneComponent.K2_GetComponentLocation` (`/Game/Blueprints/BP_Respawn.Respawn` (`self.BP_Respawn`)))))

(fn `UserConstructionScript`
  (set `self.lngSpline` (`SplineComponent.GetSplineLength` (`self.Spline`))))