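; BP_Dalle is an obstacle tile that punishes the player for crossing it at the wrong speed.
; It caches the third-person player character on BeginPlay.
; Any actor overlap checks that character's MaxWalkSpeed setting for an exact match to the required slow value, without filtering the overlapping actor.
; On a mismatch, it damages the player and teleports them to the Respawn component of a referenced respawn Blueprint.
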(event `self.ReceiveBeginPlay`
  (bind _asbp_third_person_character (cast `/Game/ThirdPerson/Blueprints/BP_ThirdPersonCharacter` (`GameplayStatics.GetPlayerCharacter` 0)))
  (set `self.AsPlayer` _asbp_third_person_character))

(event `self.ReceiveActorBeginOverlap`
  (params (OtherActor :type "Actor Object Reference"))
  ;[1 1 1] sur overlap, check la vitesse : si bonne vitesse alors rine, si mauvaise vitesse alors respawn checkpoint + dégats reçus
  (if (not (== (`CharacterMovementComponent.MaxWalkSpeed` (`Character.CharacterMovement` (`self.AsPlayer`))) 150.0))
    (`GameplayStatics.ApplyDamage` (`self.AsPlayer`) 10.0)
    (`self.K2_TeleportTo` :`self` (`self.AsPlayer`) :`DestLocation` (`SceneComponent.K2_GetComponentLocation` (`/Game/Blueprints/BP_Respawn.Respawn` (`self.Bp_Respawn`))))))

(fn `UserConstructionScript`)